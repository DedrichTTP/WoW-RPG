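; BP_Dummy is a stealth-kill target that the player can assassinate from behind.
; An overlap radius stores the third-person character and toggles a prompt widget, which turns toward the camera every tick.
; StealthBackAssin plays the death montage, hides the prompt and returns a reference location and rotation for the attacker.
; Its Ragdoll event only disables collision and grants the player XP, without simulating physics.
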(event `Ragdoll`
  ;[1 1 1] Assasinate
  (`self.SetActorEnableCollision` false)
  (`/Game/Blueprints/BPC_PlayerStats.Increase XP` (`/Game/ThirdPerson/Blueprints/BP_ThirdPersonCharacter.BPC_PlayerStats` (`self.Player Ref`)) 50.0))

(event `self.ReceiveTick`
  (params (DeltaSeconds :type "Float (single-precision)"))
  (bind _assasinate_widget (`self.Assasinate Widget`))
  ;[1 1 1] Assasinate widget
  ;;[1 1 1] Widget follow camera rot
  (`SceneComponent.K2_SetWorldRotation` _assasinate_widget (`KismetMathLibrary.FindLookAtRotation` (`SceneComponent.K2_GetComponentLocation` _assasinate_widget) (`SceneComponent.K2_GetComponentLocation` (`PlayerCameraManager.TransformComponent` (`GameplayStatics.GetPlayerCameraManager` 0)))) false false))

(event `self.Assasination Radius.OnComponentBeginOverlap`
  (params (OverlappedComponent :type "PrimitiveComponent Object Reference") (OtherActor :type "Actor Object Reference") (OtherComp :type "PrimitiveComponent Object Reference") (OtherBodyIndex :type Integer) (bFromSweep :type Boolean) (SweepResult :type "HitResult Structure (by ref)"))
  ;[1 1 1] Assasinate widget
  ;;[1 1 1] Widget visiblity
  (bind _asbp_third_person_character (cast `/Game/ThirdPerson/Blueprints/BP_ThirdPersonCharacter` OtherActor))
  (set `self.Player Ref` _asbp_third_person_character)
  (`SceneComponent.SetVisibility` (`self.Assasinate Widget`) true false))

(event `self.Assasination Radius.OnComponentEndOverlap`
  (params (OverlappedComponent :type "PrimitiveComponent Object Reference") (OtherActor :type "Actor Object Reference") (OtherComp :type "PrimitiveComponent Object Reference") (OtherBodyIndex :type Integer))
  ;[1 1 1] Assasinate widget
  ;;[1 1 1] Widget visiblity
  (cast `/Game/ThirdPerson/Blueprints/BP_ThirdPersonCharacter` OtherActor)
  (`SceneComponent.SetVisibility` (`self.Assasinate Widget`) false false))

(fn `Stealth Back Assin`
  (returns (`REF Location` :type "Vector Structure") (`REF Rotation` :type "Rotator Structure"))
  (`self.PlayAnimMontage` "/Game/Characters/Human/Male/Animations/Die.Die")
  (`self.Ragdoll`)
  (`SceneComponent.SetVisibility` (`self.Assasinate Widget`) false false)
  (return (`SceneComponent.K2_GetComponentLocation` (`self.AssassinRef`)) (`self.K2_GetActorRotation`)))

(fn `UserConstructionScript`)