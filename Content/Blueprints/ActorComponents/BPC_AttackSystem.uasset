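; Player component that runs a four-hit dual-sword melee combo with montages, sounds and hit damage.
; Attack input starts a swing or buffers the next, which SwordAttackCombo plays or StopCombo resets.
; StartSwordTrace loops a timer that sphere-traces along the right or left blade, chosen by AttackIndex.
; Hits on "Damagable" actors apply damage, camera shake and sound, throttled per blade by delayed DoOnce resets.
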(event `self.ReceiveBeginPlay`
  ;[1 1 1] Get Character Ref
  (bind _asbp_third_person_character (cast `/Game/ThirdPerson/Blueprints/BP_Player` (`self.GetOwner`)))
  (set `self.CharacterRef` _asbp_third_person_character)
  (set `self.CharacterMeshRef` (`Character.Mesh` _asbp_third_person_character)))

(event `Attack 1`
  ;[1 1 1] Combo System
  ;;[1 1 1] Attack 1
  (`|PlayMontage` (`self.CharacterMeshRef`) "/Game/Characters/Percula/Animations/Attacking/Sword_Combo_1.Sword_Combo_1"
    (:`then`
      (set `self.AttackIndex` 1))))

(event `EnhancedInput|/Game/ThirdPerson/Input/Actions/IA_Attack`
  (params (ActionValue :type Boolean) (ElapsedSeconds :type "Float (double-precision)") (TriggeredSeconds :type "Float (double-precision)") (InputAction :type "InputAction Object Reference" :default "/Game/ThirdPerson/Input/Actions/IA_Attack.IA_Attack"))
  ;[1 1 1] Combo System
  ;;[1 1 1] Attack Input
  (:`Triggered`
    (if (`self.CanAttack`)
      (`self.Sword Attack`))))

(event `Attack 2`
  ;[1 1 1] Combo System
  ;;[1 1 1] Attack 2
  (`|PlayMontage` (`self.CharacterMeshRef`) "/Game/Characters/Percula/Animations/Attacking/Sword_Combo_2.Sword_Combo_2"
    (:`then`
      (set `self.AttackIndex` 2))))

(event `Sword Attack`
  ;[1 1 1] Combo System
  ;;[1 1 1] Sword Attack
  (if (`self.IsAttacking`)
    (set `self.SaveAttack` true)
    (else
      (set `self.IsAttacking` true)
      (switch `int` (`self.AttackIndex`) :!label _label
        (:`0`
          (`self.Attack 1`))
        (:`1`
          (`self.Attack 2`))
        (:`2`
          (`self.Attack 3`))
        (:`3`
          (`self.Attack 4`)))
      (`self.Play Sword Whoosh Sounds`))))

(event `Attack 3`
  ;[1 1 1] Combo System
  ;;[1 1 1] Attack 3
  (`|PlayMontage` (`self.CharacterMeshRef`) "/Game/Characters/Percula/Animations/Attacking/Sword_Combo_3.Sword_Combo_3"
    (:`then`
      (set `self.AttackIndex` 3))))

(event `Sword Attack Combo`
  ;[1 1 1] Combo System
  ;;[1 1 1] Combo Continue
  (if (`self.SaveAttack`)
    (set `self.SaveAttack` false)
    (goto _label)
    (else
      (`self.Stop Combo`))))

(event `Attack 4`
  ;[1 1 1] Combo System
  ;;[1 1 1] Attack 4
  (`|PlayMontage` (`self.CharacterMeshRef`) "/Game/Characters/Percula/Animations/Attacking/Sword_Combo_4.Sword_Combo_4"
    (:`then`
      (set `self.AttackIndex` 4))))

(event `Stop Combo`
  ;[1 1 1] Combo System
  ;;[1 1 1] Stop Combo / Attack
  (set `self.IsAttacking` false)
  (set `self.AttackIndex` 0))

(event `Start Sword Trace`
  ;[1 1 1] Sword Trace
  (bind _returnvalue (`KismetSystemLibrary.K2_SetTimerDelegate` (delegate `Sword Trace Loop`) 0.01 true))
  (set `self.SwordTraceTimerREF` _returnvalue))

(event `Sword Trace Loop`
  (bind _characterref (`self.CharacterRef`))
  (bind _characterref_2 (`self.CharacterRef`))
  ;[1 1 1] Sword Trace
  (switch `int` (- (`self.AttackIndex`) 1)
    (:`0`
      (bind (_outhit _returnvalue) (`KismetSystemLibrary.SphereTraceSingle` :`Start` (`SceneComponent.K2_GetComponentLocation` (`/Game/ThirdPerson/Blueprints/BP_Player.SwordTopPoint_R` _characterref_2)) :`End` (`SceneComponent.K2_GetComponentLocation` (`/Game/ThirdPerson/Blueprints/BP_Player.SwordBottomPoint_R` _characterref_2)) :`Radius` 12.0 :`TraceChannel` "TraceTypeQuery1" :`DrawDebugType` "ForOneFrame" :!label _label_2))
      (if _returnvalue
        (bind (_bblockinghit _binitialoverlap _time _distance _location _impactpoint _normal _impactnormal _physmat _hitactor) (`GameplayStatics.BreakHitResult` _outhit))
        (if (`Actor.ActorHasTag` _hitactor "Damagable")
          (`/Engine/EditorBlueprintResources/StandardMacros.DoOnce` false :!label _label_3
            (:`Completed`
              (`GameplayStatics.ApplyDamage` _hitactor 32.5)
              (`GameplayStatics.PlayWorldCameraShake` "/Game/Blueprints/BP_SwordHitCameraShake.BP_SwordHitCameraShake_C" _location 0.0 2000.0)
              (`self.Play Sword Hit Sounds`)
              (`KismetSystemLibrary.Delay` 0.5)
              (goto _label_3 :!via `Reset`))))))
    (:`1`
      (bind (_outhit_2 _returnvalue_2) (`KismetSystemLibrary.SphereTraceSingle` :`Start` (`SceneComponent.K2_GetComponentLocation` (`/Game/ThirdPerson/Blueprints/BP_Player.SwordTopPoint_L` _characterref)) :`End` (`SceneComponent.K2_GetComponentLocation` (`/Game/ThirdPerson/Blueprints/BP_Player.SwordBottomPoint_L` _characterref)) :`Radius` 12.0 :`TraceChannel` "TraceTypeQuery1" :`DrawDebugType` "ForOneFrame" :`TraceColor` (struct :`R` 0.026111 :`G` 0.063934 :`B` 1.0 :`A` 1.0) :!label _label_4))
      (if _returnvalue_2
        (bind (_bblockinghit_2 _binitialoverlap_2 _time_2 _distance_2 _location_2 _impactpoint_2 _normal_2 _impactnormal_2 _physmat_2 _hitactor_2) (`GameplayStatics.BreakHitResult` _outhit_2))
        (if (`Actor.ActorHasTag` _hitactor_2 "Damagable")
          (`/Engine/EditorBlueprintResources/StandardMacros.DoOnce` false :!label _label_5
            (:`Completed`
              (`GameplayStatics.ApplyDamage` _hitactor_2 29.3)
              (`GameplayStatics.PlayWorldCameraShake` "/Game/Blueprints/BP_SwordHitCameraShake.BP_SwordHitCameraShake_C" _location_2 0.0 2000.0)
              (`self.Play Sword Hit Sounds`)
              (`KismetSystemLibrary.Delay` 0.2)
              (goto _label_5 :!via `Reset`))))))
    (:`2`
      (goto _label_4))
    (:`3`
      (goto _label_2))))

(event `Stop Sword Trace`
  ;[1 1 1] Sword Trace
  (`KismetSystemLibrary.K2_ClearAndInvalidateTimerHandle` (`self.SwordTraceTimerREF`)))

(event `Play Sword Hit Sounds`
  ;[1 1 1] Sound FX
  (`GameplayStatics.PlaySoundAtLocation` "/Game/Sound/SoundCues/SC_SwordHit.SC_SwordHit" (`Actor.K2_GetActorLocation` (`self.GetOwner`)) (struct) 1.0 1.0 0.0 "/Game/Sound/SA_Character.SA_Character" null null null))

(event `Play Sword Whoosh Sounds`
  ;[1 1 1] Sound FX
  (`GameplayStatics.PlaySoundAtLocation` "/Game/Sound/SoundCues/SC_WeaponWhoosh.SC_WeaponWhoosh" (`Actor.K2_GetActorLocation` (`self.GetOwner`)) (struct) 1.0 1.0 0.0 "/Game/Sound/SA_Character.SA_Character" null null null))

(event `Enable Weapon Collision`
  (bind _characterref (`self.CharacterRef`))
  (`PrimitiveComponent.SetCollisionProfileName` (`/Game/ThirdPerson/Blueprints/BP_Player.Weapon_L` _characterref) "PhysicsActor" true)
  (`PrimitiveComponent.SetCollisionProfileName` (`/Game/ThirdPerson/Blueprints/BP_Player.Weapon_R` _characterref) "PhysicsActor" true))