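; Actor component holding health, power, XP and level for the player or a creature, and pushing changes straight to UI widgets.
; One tick after BeginPlay it checks its owner type and initializes either the player HUD or the creature's health bar.
; Damage and power drain clamp and report depletion; XP gains trigger level-ups with a sound.
; Only damage updates creature bars; the other functions write only to player widgets.
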(event `self.ReceiveBeginPlay`
  (`KismetSystemLibrary.DelayUntilNextTick`)
  ;[1 1 1] Init Character Ref
  (bind _asbp_player (cast `/Game/ThirdPerson/Blueprints/BP_Player` (`self.GetOwner`))
    (:`then`
      (bind _output_get (set `self.PlayerREF` _asbp_player))
      (set `self.IsPlayer` true)
      (set `self.PlayerFramesREF` (`/Game/UI/Widgets/WB_HUD.WB_PlayerFrames` (`/Game/ThirdPerson/Blueprints/BP_Player.Hud REF` _output_get))))
    (:`CastFailed`
      (bind _asbp_creature_base (cast `/Game/Blueprints/BP_CreatureBase` (`self.GetOwner`)))
      (set `self.TargetREF` _asbp_creature_base)
      (set `self.IsPlayer` false)))
  ;[1 1 1] Init HP Bar
  (`ProgressBar.SetPercent` (select `bool` (`self.IsPlayer`) :`false` (`/Game/UI/Widgets/WB_FloatingHealthBar.HealthBar` (`/Game/Blueprints/BP_CreatureBase.HealthBarREF` (`self.TargetREF`))) :`true` (`/Game/UI/Frames/PlayerFrames/WB_PlayerFrames.HealthBar` (`self.PlayerFramesREF`))) (/ (`self.Current Health`) (`self.Max Health`)))
  (`TextBlock.SetText` (select `bool` (`self.IsPlayer`) :`false` (`/Game/UI/Widgets/WB_FloatingHealthBar.UnitName` (`/Game/Blueprints/BP_CreatureBase.HealthBarREF` (`self.TargetREF`))) :`true` (`/Game/UI/Frames/PlayerFrames/WB_PlayerFrames.HealthText` (`self.PlayerFramesREF`))) (`KismetTextLibrary.Conv_StringToText` (`self.Name`)))
  (if (`self.IsPlayer`)
    ;[1 1 1] Init Power Bar
    (`ProgressBar.SetPercent` (`/Game/UI/Frames/PlayerFrames/WB_PlayerFrames.PowerBar` (`self.PlayerFramesREF`)) (/ (`self.Current Power`) (`self.Max Power`)))
    ;[1 1 1] Init XP
    (`ProgressBar.SetPercent` (`/Game/UI/Widgets/WB_HUD.XPBar` (`/Game/ThirdPerson/Blueprints/BP_Player.Hud REF` (`self.PlayerREF`))) (/ (`self.Current XP`) (`self.Max XP`)))
    (`TextBlock.SetText` (`/Game/UI/Widgets/WB_HUD.XPText` (`/Game/ThirdPerson/Blueprints/BP_Player.Hud REF` (`self.PlayerREF`))) (`|FormatText` "{Current XP} / {Max XP}" (`self.Current XP`) (`self.Max XP`)))
    (`TextBlock.SetText` (`/Game/UI/Frames/PlayerFrames/WB_PlayerFrames.LevelText` (`self.PlayerFramesREF`)) (`KismetTextLibrary.Conv_IntToText` (`self.Level`)))))

(fn `Decrease Health`
  (params (Damage :type "Float (double-precision)"))
  (returns (`Is Player Dead` :type Boolean))
  (bind _current_health (`self.Current Health`))
  (if (not (<= (`self.Current Health`) 0.0))
    (bind _output_get (set `self.Current Health` (`KismetMathLibrary.FClamp` (- (`self.Current Health`) Damage) 0.0 (`self.Max Health`))))
    (`ProgressBar.SetPercent` (select `bool` (`self.IsPlayer`) :`false` (`/Game/UI/Widgets/WB_FloatingHealthBar.HealthBar` (`/Game/Blueprints/BP_CreatureBase.HealthBarREF` (`self.TargetREF`))) :`true` (`/Game/UI/Frames/PlayerFrames/WB_PlayerFrames.HealthBar` (`self.PlayerFramesREF`))) (/ _output_get (`self.Max Health`)))
    (`TextBlock.SetText` (select `bool` (`self.IsPlayer`) :`false` (`/Game/UI/Widgets/WB_FloatingHealthBar.UnitName` (`/Game/Blueprints/BP_CreatureBase.HealthBarREF` (`self.TargetREF`))) :`true` (`/Game/UI/Frames/PlayerFrames/WB_PlayerFrames.HealthText` (`self.PlayerFramesREF`))) (select `bool` (<= _current_health 0.0) :`false` (`KismetTextLibrary.Conv_IntToText` (`KismetMathLibrary.FFloor` _current_health)) :`true` "Dead"))
    (if (<= (`self.Current Health`) 0.0)
      _
      (else
        (return false))))
  (return true))

(fn `Decrease Power`
  (params (`Power Decrement` :type "Float (double-precision)"))
  (returns (`Power Drained` :type Boolean))
  (if (not (<= (`self.Current Power`) 0.0))
    (set `self.Current Power` (`KismetMathLibrary.FClamp` (- (`self.Current Power`) `Power Decrement`) 0.0 (`self.Max Power`)))
    (`ProgressBar.SetPercent` (`/Game/UI/Frames/PlayerFrames/WB_PlayerFrames.PowerBar` (`self.PlayerFramesREF`)) (/ (`self.Current Power`) (`self.Max Power`)))
    (if (<= (`self.Current Power`) 0.0)
      _
      (else
        (return false))))
  (return true))

(fn `Increase Health`
  (params (Increment :type "Float (double-precision)"))
  (set `self.Current Health` (+ (`self.Current Health`) Increment))
  (if (> (`self.Current Health`) (`self.Max Health`))
    (set `self.Current Health` (`self.Max Health`)))
  (`ProgressBar.SetPercent` (`/Game/UI/Frames/PlayerFrames/WB_PlayerFrames.HealthBar` (`self.PlayerFramesREF`)) (/ (`self.Current Health`) (`self.Max Health`)))
  (`TextBlock.SetText` (`/Game/UI/Frames/PlayerFrames/WB_PlayerFrames.HealthText` (`self.PlayerFramesREF`)) (`KismetTextLibrary.Conv_IntToText` (`KismetMathLibrary.FFloor` (`self.Current Health`)))))

(fn `Increase Level`
  (params (Increment :type Integer))
  (set `self.Level` (+ (`self.Level`) Increment))
  (set `self.Max XP` (+ (`self.Max XP`) 150.0))
  (set `self.Current XP` 0.0)
  (`TextBlock.SetText` (`/Game/UI/Frames/PlayerFrames/WB_PlayerFrames.LevelText` (`self.PlayerFramesREF`)) (`KismetTextLibrary.Conv_IntToText` (`self.Level`)))
  (`GameplayStatics.PlaySound2D` "/Game/Sound/interface/levelup.levelup" 1.0 1.0 0.0 null null))

(fn `Increase Max Health`
  (params (Increment :type "Float (double-precision)"))
  (set `self.Max Health` (+ (`self.Max Health`) Increment))
  (`ProgressBar.SetPercent` (`/Game/UI/Frames/PlayerFrames/WB_PlayerFrames.HealthBar` (`self.PlayerFramesREF`)) (/ (`self.Current Health`) (`self.Max Health`)))
  (`TextBlock.SetText` (`/Game/UI/Frames/PlayerFrames/WB_PlayerFrames.HealthText` (`self.PlayerFramesREF`)) (`KismetTextLibrary.Conv_DoubleToText` (`self.Current Health`) "HalfToEven")))

(fn `Increase Max Power`
  (params (`Power Increment` :type "Float (double-precision)"))
  (set `self.Max Power` (+ (`self.Max Power`) `Power Increment`))
  (`ProgressBar.SetPercent` (`/Game/UI/Frames/PlayerFrames/WB_PlayerFrames.PowerBar` (`self.PlayerFramesREF`)) (/ (`self.Current Power`) (`self.Max Power`))))

(fn `Increase Power`
  (params (Increment :type "Float (double-precision)"))
  (set `self.Current Power` (+ (`self.Current Power`) Increment))
  (if (> (`self.Current Power`) (`self.Max Power`))
    (set `self.Current Power` (`self.Max Power`)))
  (`ProgressBar.SetPercent` (`/Game/UI/Frames/PlayerFrames/WB_PlayerFrames.PowerBar` (`self.PlayerFramesREF`)) (/ (`self.Current Power`) (`self.Max Power`))))

(fn `Increase XP`
  (params (`XP Gain` :type "Float (double-precision)"))
  (set `self.Current XP` (+ (`self.Current XP`) `XP Gain`))
  (if (>= (`self.Current XP`) (`self.Max XP`))
    (`self.Increase Level` 1))
  (`ProgressBar.SetPercent` (`/Game/UI/Widgets/WB_HUD.XPBar` (`/Game/ThirdPerson/Blueprints/BP_Player.Hud REF` (`self.PlayerREF`))) (/ (`self.Current XP`) (`self.Max XP`)))
  (`TextBlock.SetText` (`/Game/UI/Widgets/WB_HUD.XPText` (`/Game/ThirdPerson/Blueprints/BP_Player.Hud REF` (`self.PlayerREF`))) (`|FormatText` "{Current XP} / {Max XP}" (`self.Current XP`) (`self.Max XP`))))