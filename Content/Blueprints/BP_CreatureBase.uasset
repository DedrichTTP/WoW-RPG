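; Base creature Blueprint that takes damage, can be stealth-assassinated and grants the player XP on death.
; Damage plays a random hit montage and sound, launches it along the player's facing, lowers health through its stats component and briefly shows a floating health bar.
; An overlap radius shows an assassinate prompt for a specific player gait, and StealthBackAssin kills it, returning an alignment transform.
; Widgets face the camera each tick; cursor hover applies an overlay material.
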(event `self.ReceiveBeginPlay`
  (bind _aswb_floating_health_bar (cast `/Game/UI/Widgets/WB_FloatingHealthBar` (`WidgetComponent.GetWidget` (`self.Health Bar Widget`))))
  (set `self.HealthBarREF` _aswb_floating_health_bar)
  (bind _asbp_third_person_character (cast `/Game/ThirdPerson/Blueprints/BP_Player` (`GameplayStatics.GetPlayerPawn` 0)))
  (set `self.Player Ref` _asbp_third_person_character)
  (set `PlayerController.bEnableMouseOverEvents` true (`GameplayStatics.GetPlayerController` 0)))

(event `Die`
  ;[1 1 1] Assasinate
  (`self.PlayAnimMontage` "/Game/Characters/Human/Male/Animations/Death/Die.Die")
  (`SceneComponent.SetVisibility` (`self.Health Bar Widget`) false false)
  (`/Game/Blueprints/ActorComponents/BPC_CreatureStats.Increase XP` (`/Game/ThirdPerson/Blueprints/BP_Player.BPC_CreatureStats` (`self.Player Ref`)) 50.0))

(event `self.ReceiveTick`
  (params (DeltaSeconds :type "Float (single-precision)"))
  (bind _assasinate_widget (`self.Assasinate Widget`))
  ;[1 1 1] Assasinate widget
  ;;[1 1 1] Widget follow camera rot
  (`SceneComponent.K2_SetWorldRotation` _assasinate_widget (`KismetMathLibrary.FindLookAtRotation` (`SceneComponent.K2_GetComponentLocation` _assasinate_widget) (`SceneComponent.K2_GetComponentLocation` (`PlayerCameraManager.TransformComponent` (`GameplayStatics.GetPlayerCameraManager` 0)))) false false)
  (`SceneComponent.K2_SetWorldRotation` (`self.Health Bar Widget`) (`KismetMathLibrary.FindLookAtRotation` (`SceneComponent.K2_GetComponentLocation` _assasinate_widget) (`SceneComponent.K2_GetComponentLocation` (`PlayerCameraManager.TransformComponent` (`GameplayStatics.GetPlayerCameraManager` 0)))) false false))

(event `self.Assasination Radius.OnComponentBeginOverlap`
  (params (OverlappedComponent :type "PrimitiveComponent Object Reference") (OtherActor :type "Actor Object Reference") (OtherComp :type "PrimitiveComponent Object Reference") (OtherBodyIndex :type Integer) (bFromSweep :type Boolean) (SweepResult :type "HitResult Structure (by ref)"))
  ;[1 1 1] Assasinate widget
  ;;[1 1 1] Widget visiblity
  (bind _asbp_third_person_character (cast `/Game/ThirdPerson/Blueprints/BP_Player` OtherActor))
  (if (`|EnumEquality` (`/Game/ThirdPerson/Blueprints/BP_Player.CurrentGait` _asbp_third_person_character) "NewEnumerator2")
    (`SceneComponent.SetVisibility` (`self.Assasinate Widget`) true false)))

(event `self.Assasination Radius.OnComponentEndOverlap`
  (params (OverlappedComponent :type "PrimitiveComponent Object Reference") (OtherActor :type "Actor Object Reference") (OtherComp :type "PrimitiveComponent Object Reference") (OtherBodyIndex :type Integer))
  ;[1 1 1] Assasinate widget
  ;;[1 1 1] Widget visiblity
  (cast `/Game/ThirdPerson/Blueprints/BP_Player` OtherActor)
  (`SceneComponent.SetVisibility` (`self.Assasinate Widget`) false false))

(event `self.ReceiveAnyDamage`
  (params (Damage :type "Float (single-precision)") (DamageType :type "DamageType Object Reference") (InstigatedBy :type "Controller Object Reference") (DamageCauser :type "Actor Object Reference"))
  ;[1 1 1] Receive Damage
  (if (not (`self.Dead`))
    (`self.PlayAnimMontage` (`|GetArrayItem` (`self.HitAnims`) (`KismetMathLibrary.RandomIntegerInRange` 0 (- (`KismetArrayLibrary.Array_Length` (`self.HitAnims`)) 1))))
    (`self.LaunchCharacter` (* (`KismetMathLibrary.GetForwardVector` (`self.K2_GetActorRotation` (`self.Player Ref`))) 700.0))
    (`GameplayStatics.PlaySoundAtLocation` "/Game/Sound/SoundCues/SC_HumanMale_Hit.SC_HumanMale_Hit" (`self.K2_GetActorLocation`) (struct) 1.0 1.0 0.0 null null null null)
    (`|ExecutionSequence`
      (:`then_0`
        (bind _is_player_dead (`/Game/Blueprints/ActorComponents/BPC_CreatureStats.Decrease Health` (`self.BPC_PlayerStats`) Damage))
        (if _is_player_dead
          (set `self.Dead` true)
          (`self.Die`)))
      (:`then_1`
        (`self.ShowHealthBar`)
        (`KismetSystemLibrary.K2_SetTimerDelegate` (delegate `ShowHealthBar`) 5.0)
        (`SceneComponent.SetVisibility` (`self.Health Bar Widget`) true false)))))

(event `ShowHealthBar`
  ;[1 1 1] Receive Damage
  (`SceneComponent.SetVisibility` (`self.Health Bar Widget`) false false))

(event `self.CapsuleComponent.OnBeginCursorOver`
  (params (TouchedComponent :type "PrimitiveComponent Object Reference"))
  (`MeshComponent.SetOverlayMaterial` (`self.Shoulder_R`) "/Game/UI/Materials/MAT_MouseOver.MAT_MouseOver")
  (`MeshComponent.SetOverlayMaterial` (`self.Helm`) "/Game/UI/Materials/MAT_MouseOver.MAT_MouseOver")
  (`MeshComponent.SetOverlayMaterial` (`self.Shoulder_L`) "/Game/UI/Materials/MAT_MouseOver.MAT_MouseOver")
  (`MeshComponent.SetOverlayMaterial` (`self.Mesh`) "/Game/UI/Materials/MAT_MouseOver.MAT_MouseOver"))

(event `self.CapsuleComponent.OnEndCursorOver`
  (params (TouchedComponent :type "PrimitiveComponent Object Reference"))
  (`MeshComponent.SetOverlayMaterial` (`self.Mesh`) null)
  (`MeshComponent.SetOverlayMaterial` (`self.Shoulder_R`) null)
  (`MeshComponent.SetOverlayMaterial` (`self.Helm`) null)
  (`MeshComponent.SetOverlayMaterial` (`self.Shoulder_L`) null))

(fn `GetInfo`
  (returns (Info :type "/Game/Blueprints/ActorComponents/BPC_CreatureStats Object Reference"))
  (return (`self.BPC_PlayerStats`)))

(fn `Stealth Back Assin`
  (returns (`REF Location` :type "Vector Structure") (`REF Rotation` :type "Rotator Structure"))
  (`self.Die`)
  (`SceneComponent.SetVisibility` (`self.Assasinate Widget`) false false)
  (return (`SceneComponent.K2_GetComponentLocation` (`self.AssassinRef`)) (`self.K2_GetActorRotation`)))

(fn `UserConstructionScript`)