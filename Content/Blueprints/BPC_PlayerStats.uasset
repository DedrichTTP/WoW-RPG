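; Player stats component that tracks health, power, XP and level for BP_ThirdPersonCharacter and mirrors them on its HUD.
; BeginPlay waits a tick, caches the owning character and initializes the bars and text.
; Increase and decrease functions adjust values and refresh widgets directly, with decreases returning true at zero.
; Reaching max XP raises the level, resets XP without carryover, extends the threshold and plays a sound.
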(event `self.ReceiveBeginPlay`
  (bind _hud_ref (`/Game/ThirdPerson/Blueprints/BP_ThirdPersonCharacter.Hud REF` (`self.Player Character BP`)))
  (`KismetSystemLibrary.DelayUntilNextTick`)
  ;[1 1 1] Init Character Ref
  (bind _asbp_third_person_character (cast `/Game/ThirdPerson/Blueprints/BP_ThirdPersonCharacter` (`self.GetOwner`)))
  (set `self.Player Character BP` _asbp_third_person_character)
  ;[1 1 1] Init Power Bar
  (`ProgressBar.SetPercent` (`/Game/UI/WB_HUD.PowerBar` (`/Game/ThirdPerson/Blueprints/BP_ThirdPersonCharacter.Hud REF` (`self.Player Character BP`))) (/ (`self.Current Power`) (`self.Max Power`)))
  ;[1 1 1] Init HP Bar
  (`ProgressBar.SetPercent` (`/Game/UI/WB_HUD.HealthBar` _hud_ref) (/ (`self.Current Health`) (`self.Max Health`)))
  (`TextBlock.SetText` (`/Game/UI/WB_HUD.HealthText` _hud_ref) (`KismetTextLibrary.Conv_DoubleToText` (`self.Current Health`) "HalfToEven"))
  ;[1 1 1] Init XP
  (`ProgressBar.SetPercent` (`/Game/UI/WB_HUD.XPBar` (`/Game/ThirdPerson/Blueprints/BP_ThirdPersonCharacter.Hud REF` (`self.Player Character BP`))) (/ (`self.Current XP`) (`self.Max XP`)))
  (`TextBlock.SetText` (`/Game/UI/WB_HUD.XPText` (`/Game/ThirdPerson/Blueprints/BP_ThirdPersonCharacter.Hud REF` (`self.Player Character BP`))) (`|FormatText` "{Current XP} / {Max XP}" (`self.Current XP`) (`self.Max XP`)))
  (`TextBlock.SetText` (`/Game/UI/WB_HUD.LevelText` (`/Game/ThirdPerson/Blueprints/BP_ThirdPersonCharacter.Hud REF` (`self.Player Character BP`))) (`KismetTextLibrary.Conv_IntToText` (`self.Level`))))

(fn `Decrease Health`
  (params (Damage :type "Float (double-precision)"))
  (returns (`Is Player Dead` :type Boolean))
  (bind _hud_ref (`/Game/ThirdPerson/Blueprints/BP_ThirdPersonCharacter.Hud REF` (`self.Player Character BP`)))
  (if (not (<= (`self.Current Health`) 0.0))
    (bind _output_get (set `self.Current Health` (`KismetMathLibrary.FClamp` (- (`self.Current Health`) Damage) 0.0 (`self.Max Health`))))
    (`ProgressBar.SetPercent` (`/Game/UI/WB_HUD.HealthBar` _hud_ref) (/ _output_get (`self.Max Health`)))
    (`TextBlock.SetText` (`/Game/UI/WB_HUD.HealthText` _hud_ref) (`KismetTextLibrary.Conv_IntToText` (`KismetMathLibrary.FFloor` (`self.Current Health`))))
    (if (<= (`self.Current Health`) 0.0)
      _
      (else
        (return false))))
  (return true))

(fn `Decrease Power`
  (params (`Power Decrement` :type "Float (double-precision)"))
  (returns (`Power Drained` :type Boolean))
  (if (not (<= (`self.Current Power`) 0.0))
    (set `self.Current Power` (`KismetMathLibrary.FClamp` (- (`self.Current Power`) `Power Decrement`) 0.0 (`self.Max Power`)))
    (`ProgressBar.SetPercent` (`/Game/UI/WB_HUD.PowerBar` (`/Game/ThirdPerson/Blueprints/BP_ThirdPersonCharacter.Hud REF` (`self.Player Character BP`))) (/ (`self.Current Power`) (`self.Max Power`)))
    (if (<= (`self.Current Power`) 0.0)
      _
      (else
        (return false))))
  (return true))

(fn `Increase Health`
  (params (Increment :type "Float (double-precision)"))
  (bind _hud_ref (`/Game/ThirdPerson/Blueprints/BP_ThirdPersonCharacter.Hud REF` (`self.Player Character BP`)))
  (set `self.Current Health` (+ (`self.Current Health`) Increment))
  (if (> (`self.Current Health`) (`self.Max Health`))
    (set `self.Current Health` (`self.Max Health`)))
  (`ProgressBar.SetPercent` (`/Game/UI/WB_HUD.HealthBar` _hud_ref) (/ (`self.Current Health`) (`self.Max Health`)))
  (`TextBlock.SetText` (`/Game/UI/WB_HUD.HealthText` _hud_ref) (`KismetTextLibrary.Conv_IntToText` (`KismetMathLibrary.FFloor` (`self.Current Health`)))))

(fn `Increase Level`
  (params (Increment :type Integer))
  (set `self.Level` (+ (`self.Level`) Increment))
  (set `self.Max XP` (+ (`self.Max XP`) 150.0))
  (set `self.Current XP` 0.0)
  (`TextBlock.SetText` (`/Game/UI/WB_HUD.LevelText` (`/Game/ThirdPerson/Blueprints/BP_ThirdPersonCharacter.Hud REF` (`self.Player Character BP`))) (`KismetTextLibrary.Conv_IntToText` (`self.Level`)))
  (`GameplayStatics.PlaySound2D` "/Game/Sound/interface/levelup.levelup" 1.0 1.0 0.0 null null))

(fn `Increase Max Health`
  (params (Increment :type "Float (double-precision)"))
  (bind _hud_ref (`/Game/ThirdPerson/Blueprints/BP_ThirdPersonCharacter.Hud REF` (`self.Player Character BP`)))
  (set `self.Max Health` (+ (`self.Max Health`) Increment))
  (`ProgressBar.SetPercent` (`/Game/UI/WB_HUD.HealthBar` _hud_ref) (/ (`self.Current Health`) (`self.Max Health`)))
  (`TextBlock.SetText` (`/Game/UI/WB_HUD.HealthText` _hud_ref) (`KismetTextLibrary.Conv_DoubleToText` (`self.Current Health`) "HalfToEven")))

(fn `Increase Max Power`
  (params (`Power Increment` :type "Float (double-precision)"))
  (set `self.Max Power` (+ (`self.Max Power`) `Power Increment`))
  (`ProgressBar.SetPercent` (`/Game/UI/WB_HUD.PowerBar` (`/Game/ThirdPerson/Blueprints/BP_ThirdPersonCharacter.Hud REF` (`self.Player Character BP`))) (/ (`self.Current Power`) (`self.Max Power`))))

(fn `Increase Power`
  (params (Increment :type "Float (double-precision)"))
  (set `self.Current Power` (+ (`self.Current Power`) Increment))
  (if (> (`self.Current Power`) (`self.Max Power`))
    (set `self.Current Power` (`self.Max Power`)))
  (`ProgressBar.SetPercent` (`/Game/UI/WB_HUD.PowerBar` (`/Game/ThirdPerson/Blueprints/BP_ThirdPersonCharacter.Hud REF` (`self.Player Character BP`))) (/ (`self.Current Power`) (`self.Max Power`))))

(fn `Increase XP`
  (params (`XP Gain` :type "Float (double-precision)"))
  (set `self.Current XP` (+ (`self.Current XP`) `XP Gain`))
  (if (>= (`self.Current XP`) (`self.Max XP`))
    (`self.Increase Level` 1))
  (`ProgressBar.SetPercent` (`/Game/UI/WB_HUD.XPBar` (`/Game/ThirdPerson/Blueprints/BP_ThirdPersonCharacter.Hud REF` (`self.Player Character BP`))) (/ (`self.Current XP`) (`self.Max XP`)))
  (`TextBlock.SetText` (`/Game/UI/WB_HUD.XPText` (`/Game/ThirdPerson/Blueprints/BP_ThirdPersonCharacter.Hud REF` (`self.Player Character BP`))) (`|FormatText` "{Current XP} / {Max XP}" (`self.Current XP`) (`self.Max XP`))))