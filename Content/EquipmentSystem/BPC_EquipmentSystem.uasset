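; BPC_EquipmentSystem is a player component that lets the player pick up weapons and stores their item data.
; On BeginPlay it caches the BP_Player follow camera.
; The Use input sphere-traces forward from that camera for WorldDynamic objects, and a hit BP_Weapon has its ItemData appended to WeaponSlots and is destroyed.
; A debug key prints the stored row names.
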(event Input|EnhancedActionEvents|EnhancedInputActionIA_Use
  (params (ActionValue :type Boolean) (ElapsedSeconds :type Float%20%28double-precision%29) (TriggeredSeconds :type Float%20%28double-precision%29) (InputAction :type Input%20Action%20Object%20Reference :default "/Game/ThirdPerson/Input/Actions/IA_Use.IA_Use"))
  (bind _cameraref (Variables|Default|GetCameraREF))
  (bind _returnvalue (Transformation|GetWorldLocation _cameraref))
  ;[1 1 1] Interact Trace
  (:Started
    (bind (_outhit _returnvalue_2) (Collision|SphereTraceForObjects _returnvalue (+ _returnvalue (* (Math|Vector|GetForwardVector (Transformation|GetWorldRotation _cameraref)) 1e+03)) 3e+01 (Utilities|Array|MakeArray "ObjectTypeQuery2") false 0 "ForDuration"))
    (if _returnvalue_2
      (bind _asbp_weapon (Utilities|Casting|CastToBP_Weapon (.HitActor (Collision|BreakHitResult _outhit))))
      (CallFunction|AddWeapon (Variables|/Game/EquipmentSystem/BP_Weapon.BP_Weapon_C|GetItemData _asbp_weapon))
      (Actor|DestroyActor _asbp_weapon)
      (Development|PrintString "Picked up"))))

(event EventBeginPlay
  ;[1 1 1] Get Camera Ref
  (bind _asbp_third_person_character (Utilities|Casting|CastToBP_Player (Components|GetOwner)))
  (Variables|Default|SetCameraREF (Variables|/Game/ThirdPerson/Blueprints/BP_Player.BP_Player_C|GetFollowCamera _asbp_third_person_character)))

(event Input|KeyboardEvents|DebugKeyH
  (params (Key :type Key%20Structure) (ActionValue :type Input%20Action%20Value%20Structure))
  (:Pressed
    (for _array_element (Variables|Default|GetWeaponSlots)
      (Development|PrintString (Utilities|String|ToString(Name) (.rowname (.item _array_element)))))))

(fn AddWeapon
  (params (NewItem :type S%20Slots%20Structure%20%28by%20ref%29))
  (Utilities|Array|Add (Variables|Default|GetWeaponSlots) NewItem))